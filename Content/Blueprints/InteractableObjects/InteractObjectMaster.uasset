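; InteractObjectMaster is a base Blueprint for interactable objects that can be grabbed or picked up.
; Grabbed prints the object's name, plays GrabSound at the actor's location and returns false.
; Interact checks CanInteract, prints a green success or red failure message, destroys the actor on success and returns DidInteract.
; The event graph and construction script hold no logic.
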(event EventBeginPlay)

(event Collision|EventActorBeginOverlap
  (params (OtherActor :type Actor%20Object%20Reference)))

(event EventTick
  (params (DeltaSeconds :type Float%20%28single-precision%29)))

(fn ConstructionScript)

(fn Grabbed
  (Development|PrintString (Utilities|String|Append (Utilities|String|MakeLiteralString "Grabbed: ") (Utilities|GetDisplayName self)))
  (Audio|PlaySoundatLocation (Variables|Default|GetGrabSound) (Transformation|GetActorLocation) "0, 0, 0" 1.0 1.0 0.0 0 0 0)
  (return false))

(fn Interact
  (if (Variables|Default|GetCanInteract?)
    (LocalVariables|SetDidInteract true)
    (Development|PrintString (Utilities|String|Append (Utilities|String|MakeLiteralString "Picked Up: ") (Utilities|GetDisplayName self)) true true "(R=0.147312,G=1.000000,B=0.000000,A=1.000000)")
    (Actor|DestroyActor)
    (else
      (LocalVariables|SetDidInteract false)
      (Development|PrintString (Utilities|String|Append (Utilities|String|MakeLiteralString "Can't pick up: ") (Utilities|GetDisplayName self)) true true "(R=1.000000,G=0.000000,B=0.000000,A=1.000000)")))
  (return (LocalVariables|GetDidInteract)))